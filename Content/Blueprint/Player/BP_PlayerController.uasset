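; Player controller Blueprint that handles skill casting for the player character.
; Location clicks turn the character toward the point, then fire the direction-cast dispatcher with that rotation.
; Direction casts spawn the skill row's Blueprint at the character, passing its scale and base damage.
; GetSkillsWithInput collects Enhanced Input key names for skill actions, but its skill table lookup is disconnected, leaving the returned skill list unfilled.
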(event Custom|evOnLocationClick_Event
  (params (aClickLocation :type Vector) (aSkillData :type Skill%20Data%20Row%20Structure%20%28by%20ref%29))
  (CallFunction|CastLocationSkill aClickLocation aSkillData))

(event Custom|evOnDirectionSkillCast_Event
  (params (aRotation :type Rotator) (aSkillData :type Skill%20Data%20Row%20Structure))
  (|CollapseGraph aRotation aSkillData))

(event EventBeginPlay
  (EventDispatchers|AssignEvonLocationClick (delegate Custom|evOnLocationClick_Event))
  (EventDispatchers|AssignEvonDirectionSkillCast (delegate Custom|evOnDirectionSkillCast_Event)))

(fn ConstructionScript)

(fn GetLooktoTarget
  (params (aLocation :type Vector))
  (bind _mpplayercharacter (Variables|Default|GetmpPlayerCharacter))
  (bind _returnvalue (Transformation|GetActorLocation _mpplayercharacter))
  (bind _returnvalue_2 (Math|Rotator|FindLookatRotation _returnvalue aLocation))
  (bind (_roll _pitch _yaw) (Math|Rotator|BreakRotator _returnvalue_2))
  (return (Math|Rotator|MakeRotator _roll 0.0 _yaw)))

(fn CastLocationSkill
  (params (ALocation :type Vector) (InputPin2 :type Skill%20Data%20Row%20Structure%20%28by%20ref%29))
  (bind _output_get (LocalVariables|SetRot (CallFunction|GetLooktoTarget ALocation)))
  (Transformation|SetActorRotation (Variables|Default|GetmpPlayerCharacter) _output_get)
  (Default|CallEvonDirectionSkillCast (LocalVariables|GetRot) InputPin2))

(fn GetSkillswithInput
  (Utilities|FlowControl|Sequence
    (:then_0
      ;[1 0 0.7406] Keypress
      (for _array_element (Variables|/Script/RPG_AdrianMartinez.InputConfigData|GetmpInputSkills (Variables|Default|GetmpInputData))
        (bind _returnvalue (Class|EnhancedInputSubsystemInterface|QueryKeysMappedtoAction(Message) (PlayerController|LocalPlayerSubsystems|GetEnhancedInputLocalPlayerSubsystem) _array_element))
        (Utilities|Array|Add (LocalVariables|GettKeys) (Utilities|String|ToString(Text) (Class|KismetInputLibrary|KeyGetDisplayName (Utilities|Array|Get(acopy) _returnvalue) false)))))
    (:then_1
      ;[0.4222 0.6728 1] Skills
      (for _array_element_2 (Variables|Default|GetmSkills)
        _))
    (:then_2
      (return (LocalVariables|GettKeys) (LocalVariables|GettSkills)))))