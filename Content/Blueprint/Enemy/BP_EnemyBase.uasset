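; BP_EnemyBase is an enemy Blueprint, named as a base, that gives the actor health and death on damage.
; On BeginPlay it binds a handler to its OnTakeAnyDamage event.
; The handler subtracts incoming damage from MHealth, destroys the actor at zero or below, and otherwise prints the remaining health.
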(event Custom|OnTakeAnyDamage_Event
  (params (DamagedActor :type Actor%20Object%20Reference) (Damage :type Float%20%28single-precision%29) (DamageType :type Damage%20Type%20Object%20Reference) (InstigatedBy :type Controller%20Object%20Reference) (DamageCauser :type Actor%20Object%20Reference))
  (bind _output_get (Variables|Default|SetmHealth (- (Variables|Default|GetmHealth) Damage)))
  (if (<= _output_get 0.0)
    (Actor|DestroyActor)
    (else
      (Development|PrintString (Utilities|String|ToString(Float) (Variables|Default|GetmHealth))))))

(event EventBeginPlay
  (EventDispatchers|BindEventtoOnTakeAnyDamage (delegate Custom|OnTakeAnyDamage_Event)))

(fn ConstructionScript)