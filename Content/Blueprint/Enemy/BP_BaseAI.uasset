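; BP_BaseAI is a base enemy AI controller that runs BT_BaseEnemy and writes AttackRange to its Blackboard on BeginPlay.
; Sight perception updates set CanSeePlayer from the stimulus, with no check on which actor was sensed.
; The same event sets PlayerOnRange by comparing squared distance to unsquared AttackRange, so that flag refreshes only on sight updates.
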(event OnTargetPerceptionUpdated(AIPerception)
  (params (Actor :type Actor%20Object%20Reference) (Stimulus :type AI%20Stimulus%20Structure))
  (bind _returnvalue (Class|AIPerceptionSystem|GetSenseClassforStimulus Stimulus))
  (if (== _returnvalue "/Script/AIModule.AISense_Sight")
    (AI|Components|Blackboard|SetValueasBool (AI|GetBlackboard 0) (Utilities|Name|MakeLiteralName "CanSeePlayer") (Utilities|Struct|BreakAIStimulus Stimulus))
    (AI|Components|Blackboard|SetValueasBool (AI|GetBlackboard 0) (Utilities|Name|MakeLiteralName "PlayerOnRange") (< (Class|KismetMathLibrary|VectorDistanceSquared (Transformation|GetActorLocation Actor) (Transformation|GetActorLocation (Pawn|GetControlledPawn))) (Variables|Default|GetAttackRange)))))

(event EventBeginPlay
  (AI|RunBehaviorTree "/Game/Blueprint/Enemy/BT_BaseEnemy.BT_BaseEnemy")
  (AI|Components|Blackboard|SetValueasFloat (AI|GetBlackboard 0) (Utilities|Name|MakeLiteralName "AttackRange") (Variables|Default|GetAttackRange)))

(fn ConstructionScript)